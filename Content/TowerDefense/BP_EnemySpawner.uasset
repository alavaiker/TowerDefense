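; Tower defense spawner that releases waves of enemies at its own location.
; Each EnemyWave entry sets the enemy class, count, spawn interval and initial wave delay.
; A looping timer spawns one enemy per tick, passing it the Destination's world location as Dest.
; Once the count is reached, it clears the timer, advances the index and schedules the next wave, though the bounds check allows an index equal to the array length.
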(event Custom|SpawnEnemy
  (if (>= (Variables|Default|GetSpawnedEnemies) (CallFunction|GetNumEnemies))
    (Utilities|Time|ClearandInvalidateTimerbyHandle (Variables|Default|GetTimer))
    (Math|Integer|IncrementInt (Variables|Default|GetEnemyWaveArray)
      (:%20%20
        (Variables|Default|SetSpawnedEnemies 0)
        (CallFunction|SpawnArray)))
    (else
      (CallFunction|SpawnActorEnemy))))

(event Custom|SpawnArray
  (if (not (> (Variables|Default|GetEnemyWaveArray) (Utilities|Array|Length (Variables|SpawnerConfig|GetEnemyWave))))
    (bind _returnvalue (Utilities|Time|SetTimerbyEvent (delegate Custom|SpawnEnemy) (CallFunction|GetSpawnTimer) true false (CallFunction|GetWaveTimer)))
    (Variables|Default|SetTimer _returnvalue)))

(event EventBeginPlay
  (CallFunction|SpawnArray))

(fn ConstructionScript)

(fn GetNumEnemies
  (return (.numenemies (Utilities|Array|Get(acopy) (Variables|SpawnerConfig|GetEnemyWave) (Variables|Default|GetEnemyWaveArray)))))

(fn GetEnemyType
  (return (.enemytype (Utilities|Array|Get(acopy) (Variables|SpawnerConfig|GetEnemyWave) (Variables|Default|GetEnemyWaveArray)))))

(fn GetSpawnTimer
  (return (.spawntimer (Utilities|Array|Get(acopy) (Variables|SpawnerConfig|GetEnemyWave) (Variables|Default|GetEnemyWaveArray)))))

(fn GetWaveTimer
  (return (.wavetimer (Utilities|Array|Get(acopy) (Variables|SpawnerConfig|GetEnemyWave) (Variables|Default|GetEnemyWaveArray)))))

(fn SpawnActorEnemy
  (bind _returnvalue (Game|SpawnActorfromClass (CallFunction|GetEnemyType) (Math|Transform|MakeTransform (Transformation|GetActorLocation) "0, 0, 0" "1.000000,1.000000,1.000000") "AlwaysSpawn" "MultiplyWithRoot" 0 0))
  (Math|Integer|IncrementInt (Variables|Default|GetSpawnedEnemies)
    (:%20%20
      (Variables|/Game/TowerDefense/BP_BaseEnemy.BP_BaseEnemy_C|SetDest _returnvalue (Transformation|GetWorldLocation (Variables|Default|GetDestination))))))